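; BP_NPCCharacter2 is a Pixel2D NPC that speaks once and hands out a health potion.
; When an actor with a BP_InteractionComponent overlaps its box, it plays a dialogue sound and reveals its line on a TextRender through a delayed-text macro.
; After a short pause it spawns a BP_PickUpItems potion, tosses it with a physics impulse and launch sound, then destroys the text component.
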(event `self.Box.OnComponentBeginOverlap`
  (params (OverlappedComponent :type "PrimitiveComponent Object Reference") (OtherActor :type "Actor Object Reference") (OtherComp :type "PrimitiveComponent Object Reference") (OtherBodyIndex :type Integer) (bFromSweep :type Boolean) (SweepResult :type "HitResult Structure (by ref)"))
  (`/Engine/EditorBlueprintResources/StandardMacros.IsValid` (`self.GetComponentByClass` OtherActor "/Game/Pixel2D/Blueprints/EarlyAccess/BP_InteractionComponent.BP_InteractionComponent_C")
    (:`Is Valid`
      (`/Engine/EditorBlueprintResources/StandardMacros.DoOnce` false
        (:`Completed`
          (`GameplayStatics.PlaySoundAtLocation` (`self.DialogueSound`) (`self.K2_GetActorLocation`) (struct) 1.0 1.0 0.0 null null null)
          (`/Game/Pixel2D/Blueprints/Libraries/BP_Pixel2DMacros.TextWithDelay` (`self.TextDialogue`) (`self.TextRender`) 0.03
            (:`Out`
              (`KismetSystemLibrary.Delay` 0.5)
              (bind _returnvalue (`|SpawnActorFromClass` "/Game/Pixel2D/Blueprints/Items/BP_PickUpItems.BP_PickUpItems_C" (`KismetMathLibrary.MakeTransform` (`self.K2_GetActorLocation`)) "AlwaysSpawn" "OverrideRootScale" null "/Game/Pixel2D/Blueprints/Items/BP_Item_Health_Potion.BP_Item_Health_Potion_C" "NewEnumerator0" 1 true (struct) null))
              (`PrimitiveComponent.AddImpulse` (`/Game/Pixel2D/Blueprints/Items/BP_PickUpItems.PaperFlipbook` _returnvalue) (-40.0 0.0 300.0) "None" true)
              (`GameplayStatics.PlaySoundAtLocation` (`self.LaunchSound`) (`self.K2_GetActorLocation`) (struct) 1.0 1.0 0.0 null null null)
              (`ActorComponent.K2_DestroyComponent` (`self.TextRender`)))))))))

(fn `UserConstructionScript`)